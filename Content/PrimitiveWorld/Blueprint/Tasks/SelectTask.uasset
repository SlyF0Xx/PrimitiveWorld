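; SelectTask is an AI behavior tree task that assigns the next shared task to the agent when its "current task" blackboard enum holds a specific value.
; It takes the first entry from the TaskStorage queue on NewGameState, lets it fill the blackboard via CookTask, then removes it.
; It succeeds after assignment or when the enum differs, and fails when the queue is empty.
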(event EventReceiveExecuteAI
  (params (OwnerController :type AI%20Controller%20Object%20Reference) (ControlledPawn :type Pawn%20Object%20Reference))
  (if (!= (Class|BlackboardComponent|GetValueasEnum (Class|BTFunctionLibrary|GetOwnersBlackboard) (Utilities|Name|MakeLiteralName "current task")) (Utilities|Enum|LiteralenumTasks "NewEnumerator1"))
    (AI|BehaviorTree|FinishExecute true)
    (else
      (bind _asnew_game_state (Utilities|Casting|CastToNewGameState (Game|GetGameState)))
      (if (> (Utilities|Array|Length (Variables|/Game/PrimitiveWorld/Blueprint/Tasks/TaskStorage.TaskStorage_C|Gettasks (Variables|/Game/Blueprints/NewGameState.NewGameState_C|GetTaskStorage _asnew_game_state))) 0)
        (Default|CookTask (Utilities|Array|Get(acopy) (Variables|/Game/PrimitiveWorld/Blueprint/Tasks/TaskStorage.TaskStorage_C|Gettasks (Variables|/Game/Blueprints/NewGameState.NewGameState_C|GetTaskStorage _asnew_game_state))) (Class|BTFunctionLibrary|GetOwnersBlackboard))
        (Utilities|Array|RemoveIndex (Variables|/Game/PrimitiveWorld/Blueprint/Tasks/TaskStorage.TaskStorage_C|Gettasks (Variables|/Game/Blueprints/NewGameState.NewGameState_C|GetTaskStorage _asnew_game_state)))
        (AI|BehaviorTree|FinishExecute true)
        (else
          (AI|BehaviorTree|FinishExecute false))))))