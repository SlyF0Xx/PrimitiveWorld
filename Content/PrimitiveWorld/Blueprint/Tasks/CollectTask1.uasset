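; CollectTask1 is a task actor that hands a target to an AI through its Blackboard.
; Its CookTask event writes the stored target position and object to the Blackboard and sets the current task to the first Tasks enum entry.
; The actor then destroys itself, so each instance serves as a one-shot task payload.
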(event EventBeginPlay)

(event Collision|EventActorBeginOverlap
  (params (OtherActor :type Actor%20Object%20Reference)))

(event EventTick
  (params (DeltaSeconds :type Float%20%28single-precision%29)))

(event EventCookTask
  (params (blackboard :type Blackboard%20Component%20Object%20Reference))
  (AI|Components|Blackboard|SetValueasVector blackboard (Utilities|Name|MakeLiteralName "target pos") (Variables|Default|Gettarget%20pos))
  (AI|Components|Blackboard|SetValueasObject blackboard (Utilities|Name|MakeLiteralName "target") (Utilities|ToObject(Interface) (Variables|Default|GetTargetObject)))
  (AI|Components|Blackboard|SetValueasEnum blackboard (Utilities|Name|MakeLiteralName "current task") (Utilities|Enum|LiteralenumTasks "NewEnumerator0"))
  (Actor|DestroyActor))

(fn ConstructionScript)