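; Behavior tree task that has an AI place a structure in the world.
; On execute it reads a BuildDetails object from the blackboard and passes its hit result to the blackboard's build master through PlaceStructureMessage.
; It then sets the current task enum key and finishes successfully, stopping without finishing if the BuildDetails cast fails.
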(event EventReceiveExecuteAI
  (params (OwnerController :type AI%20Controller%20Object%20Reference) (ControlledPawn :type Pawn%20Object%20Reference))
  (bind _blackboard (Variables|/Script/AIModule.AIController|GetBlackboard OwnerController))
  (bind _asbuild_details (Utilities|Casting|CastToBuildDetails (AI|Components|Blackboard|GetValueasObject _blackboard (Utilities|Name|MakeLiteralName "build hit result"))))
  (Class|IStructureBuildider|PlaceStructure(Message) (AI|Components|Blackboard|GetValueasObject _blackboard (Utilities|Name|MakeLiteralName "build master")) (Variables|/Game/PrimitiveWorld/Blueprint/Tasks/BuildDetails.BuildDetails_C|Gethit%20result _asbuild_details))
  (AI|Components|Blackboard|SetValueasEnum _blackboard (Utilities|Name|MakeLiteralName "current task") (Utilities|Enum|LiteralenumTasks "NewEnumerator1"))
  (AI|BehaviorTree|FinishExecute true))