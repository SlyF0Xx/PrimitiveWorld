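; Behavior tree task that has an AI collect resources from its blackboard target for the player.
; It gets the player character's building component through an interface and passes it, with that component's collection amount, to the target's collect-resources interface message.
; It then sets the blackboard's current task enum to a fixed value and finishes successfully.
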(event EventReceiveExecuteAI
  (params (OwnerController :type AI%20Controller%20Object%20Reference) (ControlledPawn :type Pawn%20Object%20Reference))
  (bind _blackboard (Variables|/Script/AIModule.AIController|GetBlackboard OwnerController))
  (bind _building_component (Class|PlayerBuildingGetter|GetPlayerBuildingComponent(Message) (Game|GetPlayerCharacter 0)))
  (Class|BuildingInterface|CollectResources(Message) (AI|Components|Blackboard|GetValueasObject _blackboard (Utilities|Name|MakeLiteralName "target")) _building_component (Variables|/Game/PlayerBuildingSystem/Blueprints/Components/PlayerBuildingComponent.PlayerBuildingComponent_C|GetResource%20Collection%20Amount _building_component))
  (AI|Components|Blackboard|SetValueasEnum _blackboard (Utilities|Name|MakeLiteralName "current task") (Utilities|Enum|LiteralenumTasks "NewEnumerator1"))
  (AI|BehaviorTree|FinishExecute true))