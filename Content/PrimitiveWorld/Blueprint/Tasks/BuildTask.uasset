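; BuildTask is a short-lived task actor that writes a build job into an AI Blackboard.
; CookTask asks the Blackboard's build master for a structure location and stores it as the target position.
; It wraps its HitResult in a spawned BuildDetails actor so the struct can be stored as a Blackboard object.
; It then sets the current task enum and destroys itself.
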(event EventBeginPlay)

(event Collision|EventActorBeginOverlap
  (params (OtherActor :type Actor%20Object%20Reference)))

(event EventTick
  (params (DeltaSeconds :type Float%20%28single-precision%29)))

(event EventCookTask
  (params (blackboard :type Blackboard%20Component%20Object%20Reference))
  ;[1 1 1] Get build master from BB
  (bind _location (Class|IStructureBuildider|GetStructureLocation(Message) (AI|Components|Blackboard|GetValueasObject blackboard (Utilities|Name|MakeLiteralName "build master"))))
  ;[1 1 1] Set build position based on location from build master
  (AI|Components|Blackboard|SetValueasVector blackboard (Utilities|Name|MakeLiteralName "target pos") _location)
  ;[1 1 1] Set Build hit result
  (bind _returnvalue (Game|SpawnActorfromClass "/Game/PrimitiveWorld/Blueprint/Tasks/BuildDetails.BuildDetails_C" (Math|Transform|MakeTransform "0, 0, 0") "Undefined" 0 0))
  (Variables|/Game/PrimitiveWorld/Blueprint/Tasks/BuildDetails.BuildDetails_C|Sethit%20result _returnvalue (Variables|Default|GetHit%20result))
  (AI|Components|Blackboard|SetValueasObject blackboard (Utilities|Name|MakeLiteralName "build hit result") _returnvalue)
  ;[1 1 1] Set curent task
  (AI|Components|Blackboard|SetValueasEnum blackboard (Utilities|Name|MakeLiteralName "current task") (Utilities|Enum|LiteralenumTasks "NewEnumerator2"))
  (Actor|DestroyActor))

(fn ConstructionScript)