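; TaskStorage is a task registry that creates collect and build jobs and keeps them in a Tasks list.
; CreateCollectTask spawns a CollectTask1 actor and gives it a target resource and position, while CreateBuildTask spawns a BuildTask actor carrying a hit result.
; Each task is spawned at the world origin with the storage's owner as its owner, then appended to Tasks.
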(event EventCreateBuildTask
  (params (hit%20result :type Hit%20Result%20Structure))
  (bind _returnvalue (Game|SpawnActorfromClass "/Game/PrimitiveWorld/Blueprint/Tasks/BuildTask.BuildTask_C" (Math|Transform|MakeTransform "0, 0, 0") "Undefined" (Components|GetOwner) 0))
  (Variables|/Game/PrimitiveWorld/Blueprint/Tasks/BuildTask.BuildTask_C|SetHit%20result _returnvalue hit%20result)
  (Utilities|Array|Add (Variables|Default|Gettasks) _returnvalue))

(event EventTick
  (params (DeltaSeconds :type Float%20%28single-precision%29)))

(event EventCreateCollectTask
  (params (master%20resource :type Building%20Interface%20Interface) (target%20pos :type Vector :default "0, 0, 0"))
  (bind _returnvalue (Game|SpawnActorfromClass "/Game/PrimitiveWorld/Blueprint/Tasks/CollectTask1.CollectTask1_C" (Math|Transform|MakeTransform "0, 0, 0") "Undefined" (Components|GetOwner) 0))
  (Variables|/Game/PrimitiveWorld/Blueprint/Tasks/CollectTask1.CollectTask1_C|SetTargetObject _returnvalue master%20resource)
  (Variables|/Game/PrimitiveWorld/Blueprint/Tasks/CollectTask1.CollectTask1_C|Settarget%20pos _returnvalue target%20pos)
  (Utilities|Array|Add (Variables|Default|Gettasks) _returnvalue))